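; BP_UnitManager swaps the displayed unit model between Spartan Hoplites and Triarii, using data from the Rome 2 units table.
; Each display function looks up a hard-coded row in DT_Rome2Units, sets that row's mesh on UnitModelComponent and prints a debug message.
; Nothing in this Blueprint calls either function, and the event graph holds only an unreachable test print.
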(fn ConstructionScript)

(fn DisplayUnitSpartan
  (bind _returnvalue (Utilities|GetDataTableRow "/Game/Blueprints/DT_Rome2Units.DT_Rome2Units" "SpartanHoplitesRow")
    (:then
      (Components|StaticMesh|SetStaticMesh (Variables|Default|GetUnitModel_Component) (.UnitModel (Utilities|Struct|BreakFUnitStats _returnvalue)))
      (Development|PrintString "spartan mesh fired"))))

(fn DisplayUnitTriarii
  (bind _returnvalue (Utilities|GetDataTableRow "/Game/Blueprints/DT_Rome2Units.DT_Rome2Units" "TriariiRow")
    (:then
      (Components|StaticMesh|SetStaticMesh (Variables|Default|GetUnitModel_Component) (.UnitModel (Utilities|Struct|BreakFUnitStats _returnvalue)))
      (Development|PrintString "triariimeshfired"))))